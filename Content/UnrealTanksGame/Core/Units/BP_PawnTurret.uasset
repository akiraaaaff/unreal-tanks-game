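; BP_PawnTurret is the turret unit Blueprint of the tanks game, and its graph drives a floating health bar.
; Every Tick it casts the widget component's widget to WBP_HealthBarWidget and sets the bar from the Health component's value, assuming a maximum of 100.
; It also rotates the widget component to face the player camera, billboard style.
; The graph contains no aiming or firing logic.
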(event EventBeginPlay)

(event Collision|EventActorBeginOverlap
  (params (OtherActor :type Actor%20Object%20Reference)))

(event EventTick
  (params (DeltaSeconds :type Float%20%28single-precision%29))
  (bind _health_bar_widget (Variables|Default|GetHealth%20Bar%20Widget))
  (bind _aswbp_health_bar_widget (Utilities|Casting|CastToWBP_HealthBarWidget (UserInterface|GetWidget (Variables|Default|GetHealth%20Bar%20Widget))))
  (Progress|SetPercent (Variables|/Game/UnrealTanksGame/Core/Widgets/WBP_HealthBarWidget.WBP_HealthBarWidget_C|GetHealthBar _aswbp_health_bar_widget) (/ (Variables|/Script/UnrealTanksGame.HealthComponent|GetHealth (Variables|Default|GetHealth)) 1e+02))
  (Transformation|SetWorldRotation _health_bar_widget (Math|Rotator|FindLookatRotation (Transformation|GetWorldLocation _health_bar_widget) (Transformation|GetWorldLocation (Variables|/Script/Engine.PlayerCameraManager|GetTransformComponent (Game|GetPlayerCameraManager 0)))) false false))

(fn ConstructionScript)