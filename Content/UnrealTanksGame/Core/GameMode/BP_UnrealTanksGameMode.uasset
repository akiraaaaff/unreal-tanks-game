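; BP_UnrealTanksGameMode is the tanks game mode Blueprint that drives the UI for match start, turret count and game end.
; StartGame shows a start widget, then creates and adds the HUD after a short delay.
; UpdateTurretCount writes the remaining turrets to that HUD, and GameOver adds an end widget showing a win or loss message.
; BeginPlay, Tick and the construction script are empty.
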(event EventBeginPlay)

(event EventTick
  (params (DeltaSeconds :type Float%20%28single-precision%29)))

(event EventStartGame
  (bind _returnvalue (UserInterface|CreateWidget "/Game/UnrealTanksGame/Core/Widgets/WBP_StartGameWidget.WBP_StartGameWidget_C"))
  (UserInterface|Viewport|AddtoViewport _returnvalue 0)
  (Utilities|FlowControl|Delay 3.5)
  (bind _returnvalue_2 (UserInterface|CreateWidget "/Game/UnrealTanksGame/Core/Widgets/WBP_HUDWidget.WBP_HUDWidget_C"))
  (UserInterface|Viewport|AddtoViewport _returnvalue_2 0))

(event EventGameOver
  (params (bVictory :type Boolean))
  (bind _returnvalue (UserInterface|CreateWidget "/Game/UnrealTanksGame/Core/Widgets/WBP_EndGameWidget.WBP_EndGameWidget_C"))
  (UserInterface|Viewport|AddtoViewport _returnvalue 0)
  (Rendering|Components|TextRender|SetText (Variables|/Game/UnrealTanksGame/Core/Widgets/WBP_EndGameWidget.WBP_EndGameWidget_C|GetDisplayText _returnvalue) (select bVictory "You Won!" "You Lost!")))

(event EventUpdateTurretCount
  (params (RemainingTurretCount :type Integer))
  (Rendering|Components|TextRender|SetText (Variables|/Game/UnrealTanksGame/Core/Widgets/WBP_HUDWidget.WBP_HUDWidget_C|GetTurretCountText (stale EventStartGame _returnvalue_2)) (Utilities|Text|ToText(String) (Utilities|String|Append "Turrets Remaining: " (Utilities|String|ToString(Integer) RemainingTurretCount)))))

(fn ConstructionScript)